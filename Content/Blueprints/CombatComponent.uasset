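; Combat component for battle units that drives timer-based turn requests in an ATB-style battle.
; On BeginPlay it caches the owning UnitBase and its transform, then starts an action timer whose delay shrinks as Haste rises between max and min action times.
; When the timer fires, it requests a turn from BattleGameMode.
; StartUnitTurn opens a commands widget for party units only; EndUnitTurn is empty.
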(event `self.ReceiveBeginPlay`
  (bind _asunit_base (cast `/Game/Blueprints/Units/UnitBase` (`self.GetOwner`)))
  (bind _output_get (set `self.UnitCharacter` _asunit_base))
  (set `self.BattlePosition` (`Actor.GetTransform` _output_get))
  (`self.BeginBattle`))

(fn `BeginBattle`
  (bind _minactiontime (`self.MinActionTime`))
  (bind _returnvalue (`KismetSystemLibrary.K2_SetTimer` self "RequestTurn" (+ (* (- 1.0 (`KismetMathLibrary.NormalizeToRange` (`self.Haste`) 0.0 255.0)) (- (`self.MaxActionTime`) _minactiontime)) _minactiontime)))
  (set `self.ActionTimer` _returnvalue))

(fn `EndUnitTurn`)

(fn `RequestTurn`
  (bind _asbattle_game_mode (cast `/Game/Blueprints/BattleGameMode` (`GameplayStatics.GetGameMode`)))
  (`/Game/Blueprints/BattleGameMode.TurnRequest` _asbattle_game_mode (`self.UnitCharacter`)))

(fn `StartUnitTurn`
  (bind _unitcharacter (`self.UnitCharacter`))
  (if (`KismetMathLibrary.ClassIsChildOf` (`GameplayStatics.GetObjectClass` _unitcharacter) "/Game/Blueprints/Units/PartyUnits/PartyUnitBase.PartyUnitBase_C")
    (bind _returnvalue (`|CreateWidget` "/Game/Blueprints/UI/Widgets/Actions/CommandsWidget.CommandsWidget_C" null _unitcharacter))
    (bind _output_get (set `self.CommandsWindow` _returnvalue))
    (`UserWidget.AddToViewport` _output_get 0)))