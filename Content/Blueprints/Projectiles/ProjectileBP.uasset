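; Projectile actor fired by a UnitBase, dealing combat damage to that unit's target on impact.
; On BeginPlay its Sphere ignores the instigator while moving.
; A hit spawns the impact effect, then applies damage calculated by the instigator's CombatComponent to its current UnitTarget, regardless of the actor struck.
; The projectile destroys itself after a short delay, provided the instigator cast succeeds.
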(event `self.ReceiveBeginPlay`
  (`PrimitiveComponent.IgnoreActorWhenMoving` (`self.Sphere`) (`self.GetInstigator`) true))

(event `self.ReceiveHit`
  (params (MyComp :type "PrimitiveComponent Object Reference") (Other :type "Actor Object Reference") (OtherComp :type "PrimitiveComponent Object Reference") (bSelfMoved :type Boolean) (HitLocation :type "Vector Structure") (HitNormal :type "Vector Structure") (NormalImpulse :type "Vector Structure") (Hit :type "HitResult Structure (by ref)"))
  (`GameplayStatics.SpawnEmitterAtLocation` (`self.ImpactEffect`))
  (bind _asunit_base (cast `/Game/Blueprints/Units/UnitBase` (`self.GetInstigator`)))
  (bind _combatcomponent (`/Game/Blueprints/Units/UnitBase.CombatComponent` _asunit_base))
  (bind _basedamage (`/Game/Blueprints/CombatComponent.CalculateDamage` _combatcomponent))
  (`GameplayStatics.ApplyDamage` (`/Game/Blueprints/CombatComponent.UnitTarget` _combatcomponent) _basedamage null _asunit_base (`self.Damage Type Class`))
  (`KismetSystemLibrary.Delay` 1.0)
  (`self.K2_DestroyActor`))

(fn `UserConstructionScript`)