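; ShieldBp is a defensive magic spell that temporarily buffs the stamina (STA) stat of its target unit.
; On BeginPlay it casts SpellTarget to UnitBase, looks up the bonus for its Rank in SpellPowerTable and applies it through the unit's CombatComponent.
; After a fixed 30-second delay it calls ResetTempStats, which takes no argument identifying this particular buff.
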(event `self.ReceiveBeginPlay`
  (bind _asunit_base (cast `/Game/Blueprints/Units/UnitBase` (`self.SpellTarget`)))
  (bind _combatcomponent (`/Game/Blueprints/Units/UnitBase.CombatComponent` _asunit_base))
  (`/Game/Blueprints/CombatComponent.SetRandomStatTemp` _combatcomponent (make `/Game/Blueprints/Stats/StatsModifiersStruct` 1.0 1.0 1.0 (`BlueprintMapLibrary.Map_Find` (`self.SpellPowerTable`) (`self.Rank`))))
  (`KismetSystemLibrary.Delay` 30.0)
  (`/Game/Blueprints/CombatComponent.ResetTempStats` _combatcomponent))

(fn `UserConstructionScript`
  (`parent.UserConstructionScript`))