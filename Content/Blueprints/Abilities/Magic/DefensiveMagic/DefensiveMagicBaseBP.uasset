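; DefensiveMagicBaseBP is a base Blueprint for defensive magic spells that acts on its SpellTarget as soon as it begins play.
; After the parent BeginPlay, it casts its instigator to UnitBase and has that unit's CombatComponent calculate base magic damage for the spell's class.
; It negates that value and sends it through ApplyDamage with the spell's damage type, so healing reuses the damage pipeline.
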(event `self.ReceiveBeginPlay`
  (bind _returnvalue (`self.GetInstigator`))
  (`parent.ReceiveBeginPlay`)
  (bind _asunit_base (cast `/Game/Blueprints/Units/UnitBase` _returnvalue))
  (bind _returnvalue_2 (`/Game/Blueprints/CombatComponent.CalculateMagicBaseDamage` (`/Game/Blueprints/Units/UnitBase.CombatComponent` _asunit_base) (`GameplayStatics.GetObjectClass` self)))
  (`GameplayStatics.ApplyDamage` (`self.SpellTarget`) (* _returnvalue_2 -1.0) null _returnvalue (`self.Damage Type Class`)))

(fn `UserConstructionScript`
  (`parent.UserConstructionScript`))