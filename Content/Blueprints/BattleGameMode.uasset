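; Battle game mode that sets up the fight and runs a queue of unit turns.
; On BeginPlay it switches the view to the top-down camera, gathers party and enemy units, and after a short delay adds party units to the battle HUD.
; Turn requests join a unique queue, and a DoOnce gate starts the front unit's turn through its CombatComponent.
; ReadyNextTurn reopens the gate and starts the next queued turn.
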(event `self.ReceiveBeginPlay`
  (bind _returnvalue (`GameplayStatics.GetPlayerController` 0))
  (bind _returnvalue_2 (`GameplayStatics.GetActorOfClass` "/Game/Blueprints/Camera/Camera_TopDown.Camera_TopDown_C"))
  (bind _output_get (set `self.MainBattleCamera` _returnvalue_2))
  (`PlayerController.SetViewTargetWithBlend` _returnvalue _output_get 0.0 "VTBlend_Linear" 0.0 false)
  (bind _outactors (`GameplayStatics.GetAllActorsOfClass` "/Game/Blueprints/Units/PartyUnits/PartyUnitBase.PartyUnitBase_C"))
  (set `self.PartyUnits` _outactors)
  (bind _outactors_2 (`GameplayStatics.GetAllActorsOfClass` "/Game/Blueprints/Units/EnemiesUnit/EnemyUnitBase.EnemyUnitBase_C"))
  (set `self.EnemyUnits` _outactors_2)
  (`KismetSystemLibrary.Delay` 0.2)
  (bind _asbattle_player_controller (cast `/Game/Blueprints/BattlePlayerController` _returnvalue))
  (set `self.Battle HUD` (`/Game/Blueprints/BattlePlayerController.BattleHUD` _asbattle_player_controller))
  (for _array_element (`self.PartyUnits`)
    (`/Game/Blueprints/UI/BattleHUDWidget.AddPartyUnitToHUD` (`self.Battle HUD`) _array_element)))

(event `TurnRequest`
  (params (Unit :type "/Game/Blueprints/Units/UnitBase Object Reference"))
  (`KismetArrayLibrary.Array_AddUnique` (`self.TurnOrder`) Unit)
  (`self.StartTurn`))

(event `StartTurn`
  (bind _turnorder (`self.TurnOrder`))
  (bind _combatcomponent (`/Game/Blueprints/Units/UnitBase.CombatComponent` (`|GetArrayItem` _turnorder)))
  (`/Engine/EditorBlueprintResources/StandardMacros.DoOnce` false :!label _label
    (:`Completed`
      (if (`KismetArrayLibrary.Array_IsValidIndex` _turnorder)
        (`/Game/Blueprints/CombatComponent.StartUnitTurn` _combatcomponent)
        (add `/Game/Blueprints/CombatComponent.TurnEnded` _combatcomponent (`|CreateDelegate` :!event `ReadyNextTurn`))
        (`KismetArrayLibrary.Array_Remove` _turnorder)
        (else
          (`self.ReadyNextTurn`))))))

(event `ReadyNextTurn`
  (`|ExecutionSequence`
    (:`then_0`
      (goto _label :!via `Reset`))
    (:`then_1`
      (if (`KismetArrayLibrary.Array_IsValidIndex` (`self.TurnOrder`))
        (`self.StartTurn`)))))

(fn `UserConstructionScript`)